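; Music actor that starts the music description DA_269 and plays a parameter-driven Audio component in sync with it.
; On BeginPlay it binds to the MusicSubsystem's settings-changed event, loads the description, starts playback on the next bar of the "Main" Quartz clock, and sets fixed gater and strumming parameters.
; Each settings change pushes the Chords stem's scale and root note, plus the general BPM, into the audio parameters.
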(event `self.ReceiveBeginPlay`
  (add `MusicSubsystem.OnMusicSettingsChanged` (subsystem `MusicSubsystem`) (delegate `CustomEvent`))
  (`MusicSubsystem.LoadMusicFromDescription` (subsystem `MusicSubsystem`) "/Game/Blueprints/Audio/Music/269/DA_269.DA_269")
  (bind _returnvalue (`QuartzSubsystem.GetHandleForClock` (subsystem `QuartzSubsystem`) "Main"))
  (`AudioComponent.PlayQuantized` :`self` (`self.Audio`) :`InClockHandle` _returnvalue :`InQuantizationBoundary` (make `QuartzQuantizationBoundary` "Bar" 1.0 "TransportRelative"))
  (`AudioParameterControllerInterface.SetFloatParameter` (`self.Audio`) "GaterAmount" 0.6)
  (`AudioParameterControllerInterface.SetFloatParameter` (`self.Audio`) "NormalizedStrummingVelocity" 0.6))

(event `CustomEvent`
  (params (NewMusicDescription :type "DAMusicDescription Object Reference"))
  (bind ((`RootNote` _rootnote) (`Scale` _scale)) (break `StemDescription` (`BlueprintMapLibrary.Map_Find` (`DAMusicDescription.Stems` NewMusicDescription) "Chords")))
  (`AudioComponent.SetIntParameter` (`self.Audio`) "ScaleIndex" (`KismetMathLibrary.Conv_ByteToInt` (`KismetSystemLibrary.MakeLiteralByte` _scale)))
  (`AudioParameterControllerInterface.SetFloatParameter` (`self.Audio`) "RootNote" (`KismetMathLibrary.Conv_ByteToDouble` (`KismetSystemLibrary.MakeLiteralByte` _rootnote)))
  (`AudioParameterControllerInterface.SetFloatParameter` (`self.Audio`) "BPM" (`KismetMathLibrary.Conv_IntToDouble` (`DAMusicDescription.GeneralBPM` NewMusicDescription))))

(fn `UserConstructionScript`)